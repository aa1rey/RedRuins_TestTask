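; BP_MechanicArm is a mechanical arm Blueprint built around a cable component.
; On BeginPlay it attaches the cable's end to a configured component and socket.
; UpdateLength sets the cable length, capped at MaxLength.
; MainAction is an empty stub, and AltAction only prints Start or End based on an in-progress flag.
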(event `self.ReceiveBeginPlay`
  (`CableComponent.SetAttachEndToComponent` (`self.Cable`) (`self.Component`) (`self.Socket Name`)))

(event `/Game/Task_07/BPI_Actions.MainAction`)

(event `/Game/Task_07/BPI_Actions.AltAction`
  (bind _output_get (set `self.bAltActionInProgress` (`self.bAltActionInProgress`)))
  (if _output_get
    (`KismetSystemLibrary.PrintString` "Start")
    (else
      (`KismetSystemLibrary.PrintString` "End"))))

(fn `Update Length`
  (params (NewLength :type "Float (double-precision)"))
  (bind _maxlength (`self.MaxLength`))
  (set `CableComponent.CableLength` (select `bool` (<= NewLength _maxlength) :`false` _maxlength :`true` NewLength :!type "Float (single-precision)") (`self.Cable`)))

(fn `UserConstructionScript`)