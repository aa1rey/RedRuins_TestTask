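; Interactable sphere actor that changes color on interaction and shows a screen-space marker with its distance to the player.
; While a character overlaps its collider, a looping timer line-traces to it to decide whether interaction is blocked.
; Tick projects the marker to screen when marked, clamping it to the viewport.
; Event dispatchers feed blocking, overlap, distance and clamp state to the label and marker widgets.
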(event `self.ReceiveBeginPlay`
  (bind _wmarkerclass (`self.WMarkerClass`))
  (bind _returnvalue (`KismetMaterialLibrary.CreateDynamicMaterialInstance` (`PrimitiveComponent.GetMaterial` (`self.Sphere`) 0)))
  (bind _output_get (set `self.DMI_Sphere` _returnvalue))
  (`PrimitiveComponent.SetMaterial` (`self.Sphere`) 0 _output_get)
  (`MaterialInstanceDynamic.SetVectorParameterValue` (`self.DMI_Sphere`) "BaseColor" (`self.InteractionColorBefore`))
  (bind _w_interact_label (`self.W_Interact_Label`)
    (:`then`
      (bind _asw_interact_lable (cast `/Game/Task_01/Widgets/W_Interact_Lable` (`WidgetComponent.GetWidget` _w_interact_label)))
      (add `self.OnInteractionBlocking` (`|CreateDelegate` _asw_interact_lable :!event `OnOverlapInteractiveObject`))
      (if (`KismetSystemLibrary.IsValidClass` _wmarkerclass)
        (bind _returnvalue_2 (`|CreateWidget` _wmarkerclass (`GameplayStatics.GetPlayerController` 0)))
        (bind _output_get_2 (set `self.MarkerWidget` _returnvalue_2))
        (`Widget.SetRenderTransformPivot` _output_get_2 (0.5 0.5))
        (`UserWidget.AddToViewport` (`self.MarkerWidget`) 0)
        (`self.Set Widget Position on Screen`)
        (bind _asw_marker (cast `/Game/Task_01/Widgets/W_Marker` (`self.MarkerWidget`)))
        (`|ExecutionSequence`
          (:`then_0`
            (add `self.OnCharacterOverlaping` (`|CreateDelegate` _asw_marker :!event `OnCharacterOverlaping`)))
          (:`then_1`
            (add `self.OnDistanceToCharacterUpdate` (`|CreateDelegate` _asw_marker :!event `OnDistanceUpdate`)))
          (:`then_2`
            (add `self.OnMarkerClampedInViewport` (`|CreateDelegate` _asw_marker :!event `OnClampedInViewport`))))))
    (:`else`)))

(event `self.OverlapColider.OnComponentBeginOverlap`
  (params (OverlappedComponent :type "PrimitiveComponent Object Reference") (OtherActor :type "Actor Object Reference") (OtherComp :type "PrimitiveComponent Object Reference") (OtherBodyIndex :type Integer) (bFromSweep :type Boolean) (SweepResult :type "HitResult Structure (by ref)"))
  ;[0 0 0] Set overlaped character and start checking blocking objects between him and this
  (bind _asbp_task_04_character (cast `/Game/Task_01/Blueprints/BP_Task_1_Character` OtherActor))
  (set `self.OverlapedCharacter` _asbp_task_04_character)
  (bind _returnvalue (`KismetSystemLibrary.K2_SetTimerDelegate` (`|CreateDelegate` :!event `DoesInteractionBlocked`) 0.1 true))
  (set `self.InteractionBlockedTimerHandle` _returnvalue)
  (`self.OnCharacterOverlaping` true))

(event `self.OverlapColider.OnComponentEndOverlap`
  (params (OverlappedComponent :type "PrimitiveComponent Object Reference") (OtherActor :type "Actor Object Reference") (OtherComp :type "PrimitiveComponent Object Reference") (OtherBodyIndex :type Integer))
  ;[0 0 0] Stop check for blocking interaction and clear overlaped character from memory
  (bind _overlapedcharacter (`self.OverlapedCharacter`)
    (:`then`
      (if (== _overlapedcharacter OtherActor)
        (`KismetSystemLibrary.K2_ClearAndInvalidateTimerHandle` (`self.InteractionBlockedTimerHandle`))
        (`self.OnInteractionBlocking` true)
        (set `self.OverlapedCharacter` null)
        (`self.OnCharacterOverlaping` false)))
    (:`else`)))

(event `/Game/Task_01/Blueprints/BPI_Interaction.Interaction`
  ;[0 0 0] Change material color to red on interaction
  (if (not (`self.bDoesInteractionBlocking`))
    (`MaterialInstanceDynamic.SetVectorParameterValue` (`self.DMI_Sphere`) "BaseColor" (`self.InteractionColorAfter`))))

(event `self.ReceiveTick`
  (params (DeltaSeconds :type "Float (single-precision)"))
  (`|ExecutionSequence`
    (:`then_0`
      (if (and (`self.bMarked`) true)
        (`self.Set Widget Position on Screen`)
        (`self.OnDistanceToCharacterUpdate` (`KismetMathLibrary.Round` (/ (`KismetMathLibrary.Vector_Distance` (`self.K2_GetActorLocation`) (`self.K2_GetActorLocation` (`GameplayStatics.GetPlayerCharacter` 0))) 100.0)))))))

(fn `DoesInteractionBlocked`
  (bind _overlapedcharacter (`self.OverlapedCharacter`)
    (:`then`
      (bind (_outhit _returnvalue) (`KismetSystemLibrary.LineTraceSingle` (`self.K2_GetActorLocation`) (`self.K2_GetActorLocation` _overlapedcharacter) "TraceTypeQuery1"))
      (bind _output_get (set `self.bDoesInteractionBlocking` (and _returnvalue (not (== (`.HitActor` (`GameplayStatics.BreakHitResult` _outhit)) _overlapedcharacter)))))
      (`self.OnInteractionBlocking` _output_get)
      (return))
    (:`else`
      (`KismetSystemLibrary.K2_ClearAndInvalidateTimerHandle` (`self.InteractionBlockedTimerHandle`))
      (return))))

(fn `Set Widget Position on Screen`
  (bind (_returnvalue_x _returnvalue_y) (`KismetMathLibrary.BreakVector2D` (`WidgetLayoutLibrary.GetViewportSize`)))
  (bind _offsetposition (`self.OffsetPosition`))
  (bind _screenlocation (`PlayerController.ProjectWorldLocationToScreen` (`GameplayStatics.GetPlayerController` 0) (`self.K2_GetActorLocation`) false))
  (bind _returnvalue (/ _offsetposition 2.0))
  (bind _returnvalue_2 (+ _returnvalue_y _offsetposition))
  (bind _returnvalue_3 (+ _returnvalue_x _offsetposition))
  (bind _returnvalue_4 (+ (`.Y` (`KismetMathLibrary.BreakVector2D` _screenlocation)) _returnvalue))
  (bind _returnvalue_5 (+ (`KismetMathLibrary.BreakVector2D` _screenlocation) _returnvalue))
  (bind _markerwidget (`self.MarkerWidget`)
    (:`then`
      (`UserWidget.SetPositionInViewport` _markerwidget (`KismetMathLibrary.MakeVector2D` (`KismetMathLibrary.FClamp` _returnvalue_5 0.0 _returnvalue_3) (`KismetMathLibrary.FClamp` _returnvalue_4 0.0 _returnvalue_2)) true)
      (`self.OnMarkerClampedInViewport` (not (and (`KismetMathLibrary.InRange_FloatFloat` _returnvalue_5 0.0 _returnvalue_3) (`KismetMathLibrary.InRange_FloatFloat` _returnvalue_4 0.0 _returnvalue_2))))
      (return))
    (:`else`
      (return))))

(fn `UserConstructionScript`)