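; BP_Task_06_Actor is an actor that uses a ProjectileMovement component to home in on a Target.
; On BeginPlay, if Target is valid, it assigns one of the target's scene components as the homing target, leaving steering to that component.
; The SteeringMovement function and construction script are empty, and leftover math-expression nodes for rotating the actor's location with sine and cosine are unused.
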(event `self.ReceiveBeginPlay`
  (bind _target (`self.Target`))
  ;[0 0 0] Set target
  (`/Engine/EditorBlueprintResources/StandardMacros.IsValid` _target
    (:`Is Valid`
      (set `ProjectileMovementComponent.HomingTargetComponent` (`self.GetComponentByClass` _target "/Script/Engine.SceneComponent") (`self.ProjectileMovement`)))))

(fn `SteeringMovement`)

(fn `UserConstructionScript`)