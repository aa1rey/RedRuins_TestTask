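; Task 4 character Blueprint for experimenting with replication of spawned actors and runtime-created components.
; On server BeginPlay, SpawnServer calls SpawnMulti to spawn and store a BP_ActorForReplication, whose Value prints every Tick and rises through ChangeReplicatedValues.
; CreateDynamicComponent adds a static mesh component, snaps it to the head socket and prints its name.
; Disconnected graphs retain an abandoned UObject replication attempt, noted as not working.
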(event `SpawnServer`
  (`self.SpawnMulti`))

(event `SpawnMulti`
  (`|ExecutionSequence`
    (:`then_0`
      (bind _returnvalue (`|SpawnActorFromClass` "/Game/Task_04/BP_ActorForReplication.BP_ActorForReplication_C" (`KismetMathLibrary.MakeTransform` (0.0 0.0 0.0)) "Undefined" "MultiplyWithRoot" null 20.0 null))
      (set `self.NewVar` _returnvalue))))

(event `self.ReceiveBeginPlay`
  (if (`KismetSystemLibrary.IsServer`)
    (`self.SpawnServer`)))

(event `self.ReceiveTick`
  (params (DeltaSeconds :type "Float (single-precision)"))
  (`|ExecutionSequence`
    (:`then_0`
      (bind _newvar (`self.NewVar`)
        (:`then`
          (`KismetSystemLibrary.PrintString` (`KismetStringLibrary.Conv_DoubleToString` (`/Game/Task_04/BP_ActorForReplication.value` _newvar)) true true (struct :`G` 0.66 :`B` 1.0 :`A` 1.0) 0.0))
        (:`else`)))))

(event `ChangeReplicatedValues`
  (`|ExecutionSequence`
    (:`then_0`
      (bind _newvar (`self.NewVar`)
        (:`then`
          (set `/Game/Task_04/BP_ActorForReplication.value` (+ (`/Game/Task_04/BP_ActorForReplication.value` _newvar) 10.0) _newvar))
        (:`else`)))))

(event `Create Dynamic Component`
  ;[0 0 0] Create Dynamic Component
  (bind _returnvalue (`AddComponent|NODE_AddStaticMeshComponent-0` :`bManualAttachment` true :`RelativeTransform` (`SceneComponent.GetSocketTransform` (`self.Mesh`) "head" "RTS_Actor")))
  (bind _output_get (set `self.Rep_DynamicComponent` _returnvalue))
  (`StaticMeshComponent.SetStaticMesh` _output_get "/Engine/VREditor/TransformGizmo/UniformScaleHandle.UniformScaleHandle")
  (`SceneComponent.K2_AttachToComponent` _output_get (`self.Mesh`) "head" "SnapToTarget" "SnapToTarget" "SnapToTarget" true)
  (`KismetSystemLibrary.PrintString` (`KismetSystemLibrary.GetDisplayName` (`self.Rep_DynamicComponent`)) true true (struct :`R` 1.0 :`G` 0.59945 :`A` 1.0) 100.0))

(fn `UserConstructionScript`
  (`parent.UserConstructionScript`))