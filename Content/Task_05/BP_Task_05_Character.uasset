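; Character that rides a looping spline and fires projectiles along a predicted arc.
; A looping timer advances the spline distance by an input-adjusted, clamped acceleration, wrapping to the start at the end.
; While aiming, another timer pitches the projectile socket with the camera, predicts and draws the path, and moves a hit marker to the impact point.
; Launching stops prediction and spawns a projectile with the predicted velocity.
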(event `self.ReceiveBeginPlay`
  (`self.BeginSplineMovement`)
  (bind _returnvalue (`|SpawnActorFromClass` (`self.HitPlaceMarkerClass`) (`KismetMathLibrary.MakeTransform` (0.0 0.0 -10000.0)) "AlwaysSpawn" "MultiplyWithRoot" null null))
  (bind _output_get (set `self.HitPlaceMarkerRef` _returnvalue))
  (`self.SetActorHiddenInGame` _output_get true))

(event `/Game/Task_05/BPI_SplineMovement.AccelerateSplineMovement`
  (params (Axis :type "Float (double-precision)"))
  ;[0 0 0] Set spline movement acceleration
  (set `self.Acceleration` (`KismetMathLibrary.FClamp` (+ (/ Axis (`self.AccelerationHardness`)) (`self.Acceleration`)) (`self.MinAcceleration`) (`self.MaxAcceleration`))))

(event `MoveAlongSpline`
  (bind _returnvalue (+ (`self.CurrentDistanceOnSpline`) (`self.Acceleration`)))
  (bind _returnvalue_2 (`SplineComponent.GetSplineLength` (`/Game/Task_05/BP_MovementPath.Spline` (`self.SplineRef`))))
  ;[0 0 0] Spline Movement
  (bind _output_get (set `self.CurrentDistanceOnSpline` (`KismetMathLibrary.FInterpTo_Constant` (select `bool` (<= _returnvalue _returnvalue_2) :`true` _returnvalue :!type "Float (single-precision)") _returnvalue_2 (`GameplayStatics.GetWorldDeltaSeconds`) 0.5)))
  (bind (_returnvalue_x _returnvalue_y _returnvalue_z) (`KismetMathLibrary.BreakVector` (`SplineComponent.GetLocationAtDistanceAlongSpline` (`/Game/Task_05/BP_MovementPath.Spline` (`self.SplineRef`)) _output_get "World")))
  (`self.K2_SetActorLocation` (`KismetMathLibrary.MakeVector` _returnvalue_x _returnvalue_y (+ _returnvalue_z 158.0))))

(event `/Game/Task_05/BPI_TrajectoryLaunch.BeginPredictTrajectory`
  ;[0 0 0] Begin Predict Trajectory
  (bind _returnvalue (`KismetSystemLibrary.K2_SetTimerDelegate` (`|CreateDelegate` :!event `PredictTrajectory`) 0.01 true))
  (set `self.PredictTrajectoryTimerHandle` _returnvalue)
  (bind _hitplacemarkerref (`self.HitPlaceMarkerRef`)
    (:`then`
      (`self.SetActorHiddenInGame` _hitplacemarkerref false))
    (:`else`)))

(event `PredictTrajectory`
  (bind (_returnvalue_roll _returnvalue_pitch _returnvalue_yaw) (`KismetMathLibrary.BreakRotator` (`SceneComponent.K2_GetComponentRotation` (`self.ProjectileSocket`))))
  (bind (_returnvalue_roll_2 _returnvalue_pitch_2) (`KismetMathLibrary.BreakRotator` (`SceneComponent.K2_GetComponentRotation` (`self.Camera`))))
  (bind (_returnvalue_location _returnvalue_rotation) (`KismetMathLibrary.BreakTransform` (`SceneComponent.GetSocketTransform` (`self.ProjectileSocket`) "None" "RTS_World")))
  ;[0 0 0] Predict Trajectory
  ;;[0.04688 0.04688 0.04688] Rotate projectile socket with camera
  (`SceneComponent.K2_SetWorldRotation` (`self.ProjectileSocket`) (`KismetMathLibrary.MakeRotator` _returnvalue_roll _returnvalue_pitch_2 _returnvalue_yaw) false false)
  (bind _predictresult (`GameplayStatics.Blueprint_PredictProjectilePath_Advanced` (make `PredictProjectilePathParams` _returnvalue_location (* (`KismetMathLibrary.GetForwardVector` _returnvalue_rotation) (`self.ProjectileLaunchSpeed`)) true (`self.Predict Projectile Sphere Radius`) 3.0 true "ECC_WorldStatic" _ (`|MakeArray` (`self.ProjectileRef`)) 15.0 0.0 "ForDuration" 0.01)))
  ;;[0.03646 0.03646 0.03646] Geting the location of the hit along the trajectory and set it to the marker location
  (set `self.ProjectileHitLocation` (`.ImpactPoint` (`GameplayStatics.BreakHitResult` (`.HitResult` (break `PredictProjectilePathResult` _predictresult)))))
  (set `self.PredictedProjectileVelocity` (`.Velocity` (break `PredictProjectilePathPointData` (`|GetArrayItem` (break `PredictProjectilePathResult` _predictresult)))))
  (bind _hitplacemarkerref (`self.HitPlaceMarkerRef`)
    (:`then`
      (`self.K2_SetActorLocation` _hitplacemarkerref (`self.ProjectileHitLocation`) false false))
    (:`else`)))

(event `/Game/Task_05/BPI_TrajectoryLaunch.EndPredictTrajectory`
  ;[0 0 0] End Predict Trajectory
  (`KismetSystemLibrary.K2_ClearAndInvalidateTimerHandle` (`self.PredictTrajectoryTimerHandle`)))

(event `/Game/Task_05/BPI_TrajectoryLaunch.Launch Along Trajectory`
  (bind _returnvalue_location (`KismetMathLibrary.BreakTransform` (`SceneComponent.K2_GetComponentToWorld` (`self.ProjectileSocket`))))
  ;[0 0 0] Launch projectile with calculated velocity
  (`self.EndPredictTrajectory`)
  (bind _returnvalue (`|SpawnActorFromClass` (`self.ProjectileClass`) (`KismetMathLibrary.MakeTransform` _returnvalue_location) "AlwaysSpawn" "MultiplyWithRoot" null null))
  (bind _output_get (set `self.ProjectileRef` _returnvalue))
  (message `/Game/Task_05/BPI_ProjectileLaunch.LaunchProjectile` _output_get (`self.PredictedProjectileVelocity`)))

(fn `BeginSplineMovement`
  (returns (`Success?` :type Boolean))
  (bind _splineref (`self.SplineRef`)
    (:`then`
      (set `self.CurrentDistanceOnSpline` (`SplineComponent.GetDistanceAlongSplineAtLocation` (`/Game/Task_05/BP_MovementPath.Spline` _splineref) (`self.K2_GetActorLocation`) "World"))
      (bind _returnvalue (`KismetSystemLibrary.K2_SetTimerDelegate` (`|CreateDelegate` :!event `MoveAlongSpline`) 0.01 true))
      (set `self.SplineMovementTimerHandle` _returnvalue)
      (return true))
    (:`else`
      (return false))))

(fn `EndSplineMovement`
  (`KismetSystemLibrary.K2_ClearAndInvalidateTimerHandle` (`self.SplineMovementTimerHandle`))
  (return))

(fn `UserConstructionScript`)